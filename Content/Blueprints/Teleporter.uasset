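; Teleporter with a trigger box that moves the overlapping actor to a set end location and rotation behind a screen transition.
; On overlap it disables input and camera boom collision testing, plays the FadeIn level sequence, and waits briefly before moving the actor.
; It then sets control rotation from the camera boom with a downward pitch offset, plays FadeOut, and restores input and collision testing.
; The overlapping actor is not checked to be the player.
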(event `self.Box.OnComponentBeginOverlap`
  (params (OverlappedComponent :type "PrimitiveComponent Object Reference") (OtherActor :type "Actor Object Reference") (OtherComp :type "PrimitiveComponent Object Reference") (OtherBodyIndex :type Integer) (bFromSweep :type Boolean) (SweepResult :type "HitResult Structure (by ref)"))
  (bind _returnvalue (`GameplayStatics.GetPlayerController` 0))
  (bind _asbp_third_person_character (cast `/Game/ThirdPerson/Blueprints/BP_ThirdPersonCharacter` (`GameplayStatics.GetPlayerCharacter` 0)))
  (set `SpringArmComponent.bDoCollisionTest` false (`/Game/ThirdPerson/Blueprints/BP_ThirdPersonCharacter.CameraBoom` _asbp_third_person_character))
  (`self.DisableInput` OtherActor (`GameplayStatics.GetPlayerController` 0))
  (bind (_outactor _returnvalue_2) (`LevelSequencePlayer.CreateLevelSequencePlayer` (`self.FadeIn`)))
  (`MovieSceneSequencePlayer.Play` _returnvalue_2)
  (`KismetSystemLibrary.Delay` 1.5)
  (`self.K2_SetActorTransform` OtherActor (`KismetMathLibrary.MakeTransform` (`self.EndLoc`) (`self.EndLocRot`)) false false)
  (bind _asbp_third_person_character_2 (cast `/Game/ThirdPerson/Blueprints/BP_ThirdPersonCharacter` (`GameplayStatics.GetPlayerCharacter` 0)))
  (bind _cameraboom (`/Game/ThirdPerson/Blueprints/BP_ThirdPersonCharacter.CameraBoom` _asbp_third_person_character_2))
  (`Controller.SetControlRotation` _returnvalue (`KismetMathLibrary.MakeRotator` (.roll (`KismetMathLibrary.RLerp` (`SceneComponent.K2_GetComponentRotation` _cameraboom) (`Controller.GetControlRotation` _returnvalue) 0.0 true)) (+ (.pitch (`KismetMathLibrary.RLerp` (`SceneComponent.K2_GetComponentRotation` _cameraboom) (`Controller.GetControlRotation` _returnvalue) 0.0 true)) -30.0) (.yaw (`KismetMathLibrary.RLerp` (`SceneComponent.K2_GetComponentRotation` _cameraboom) (`Controller.GetControlRotation` _returnvalue) 0.0 true))))
  (bind (_outactor_2 _returnvalue_3) (`LevelSequencePlayer.CreateLevelSequencePlayer` (`self.FadeOut`)))
  (`MovieSceneSequencePlayer.Play` _returnvalue_3)
  (`self.EnableInput` OtherActor (`GameplayStatics.GetPlayerController` 0))
  (set `SpringArmComponent.bDoCollisionTest` true _cameraboom))

(fn `UserConstructionScript`)