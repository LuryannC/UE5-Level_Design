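; Lift is a Blueprint that slides two door actors open when its Box trigger is overlapped and closes them when the overlap ends, unless Locked.
; BeginPlay caches each door's location, and two timelines lerp each door from there by its EndPoint offset, reversing to close.
; Each direction swaps the Audio sound, with closing playback starting partway in.
; An unconnected loop that negates the EndPoint offsets never runs.
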(event `self.ReceiveBeginPlay`
  (for (_array_element _array_index) (`self.Doors`)
    (`KismetArrayLibrary.Array_Set` (`self.StartPoint`) _array_index (`self.K2_GetActorLocation` _array_element))))

(event `self.Box.OnComponentBeginOverlap`
  (params (OverlappedComponent :type "PrimitiveComponent Object Reference") (OtherActor :type "Actor Object Reference") (OtherComp :type "PrimitiveComponent Object Reference") (OtherBodyIndex :type Integer) (bFromSweep :type Boolean) (SweepResult :type "HitResult Structure (by ref)"))
  (bind _doors (`self.Doors`))
  (bind _audio (`self.Audio`))
  (bind _output (`|GetArrayItem` (`self.StartPoint`) 1))
  (bind _output_2 (`|GetArrayItem` (`self.StartPoint`)))
  (if (not (`self.Locked?`))
    (`AudioComponent.SetSound` _audio (`|GetArrayItem` (`self.Sounds`) 1))
    (`AudioComponent.Play` _audio 0.0)
    (`|ExecutionSequence`
      (:`then_0`
        (bind (_direction _newtrack_0) (`Timeline|Timeline_0` :!label _label)
          (:`Update`
            (`self.K2_SetActorLocation` (`|GetArrayItem` _doors) (`KismetMathLibrary.VLerp` _output_2 (+ _output_2 (`|GetArrayItem` (`self.EndPoint`))) _newtrack_0) false false))))
      (:`then_1`
        (bind (_direction_2 _newtrack_0_2) (`Timeline|Timeline_1` :!label _label_2)
          (:`Update`
            (`self.K2_SetActorLocation` (`|GetArrayItem` _doors 1) (`KismetMathLibrary.VLerp` _output (+ _output (`|GetArrayItem` (`self.EndPoint`) 1)) _newtrack_0_2) false false)))))))

(event `self.Box.OnComponentEndOverlap`
  (params (OverlappedComponent :type "PrimitiveComponent Object Reference") (OtherActor :type "Actor Object Reference") (OtherComp :type "PrimitiveComponent Object Reference") (OtherBodyIndex :type Integer))
  (bind _audio (`self.Audio`))
  (if (not (`self.Locked?`))
    (`AudioComponent.SetSound` _audio (`|GetArrayItem` (`self.Sounds`)))
    (`AudioComponent.Play` _audio 2.2)
    (`|ExecutionSequence`
      (:`then_0`
        (goto _label :!via `Reverse`))
      (:`then_1`
        (goto _label_2 :!via `Reverse`)))))

(fn `UserConstructionScript`)